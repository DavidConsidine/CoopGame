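; Grenade projectile actor that detonates on a fixed timer started at BeginPlay, with no impact trigger in its graphs.
; The Explode event spawns an explosion particle effect, applies radial damage credited to the instigator's controller, and destroys the actor.
; A debug sphere showing the damage radius is drawn after the DestroyActor call.
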(event Custom|Explode
  (bind _returnvalue (Transformation|GetActorLocation))
  (Effects|SpawnEmitteratLocation "/Game/WeaponEffects/Explosion/P_Explosion.P_Explosion" _returnvalue)
  (Game|Damage|ApplyRadialDamage 1e+02 _returnvalue (Variables|Default|GetDamageRadius) 0 0 self (Game|GetInstigatorController) false "ECC_Visibility")
  (Actor|DestroyActor)
  (Rendering|Debug|DrawDebugSphere _returnvalue (Variables|Default|GetDamageRadius) 12 "(R=1.000000,G=0.842126,B=0.000000,A=1.000000)" 1.0 2.0))

(event EventBeginPlay
  (Utilities|FlowControl|Delay 1.0)
  (CallFunction|Explode))

(fn ConstructionScript)