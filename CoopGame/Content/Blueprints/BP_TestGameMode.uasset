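; Test game mode that spawns tracker bots at locations chosen by an environment query.
; SpawnNewBot runs the spawn-location EQS query with the game mode as querier, picking randomly from the best 25 percent.
; On query success, each returned location gets a brief debug sphere and a BP_TrackerBot, adjusted to avoid collision or skipped if blocked.
; Each spawn attempt prints the bot's display name for debugging.
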(event Custom|OnQueryFinishedEvent_Event_0
  (params (QueryInstance :type Env%20Query%20Instance%20Blueprint%20Wrapper%20Object%20Reference) (QueryStatus :type EEnvQueryStatus%20Enum :default "Processing"))
  (switch Utilities|FlowControl|Switch|SwitchonEEnvQueryStatus QueryStatus
    (:Success
      (for _array_element (Class|EnvQueryInstanceBlueprintWrapper|GetResultsasLocations QueryInstance)
        (Rendering|Debug|DrawDebugSphere _array_element 5e+01 12 "(R=1.000000,G=0.941159,B=0.000000,A=1.000000)" 2.0 2.0)
        (bind _returnvalue (Game|SpawnActorfromClass "/Game/TrackerBot/BP_TrackerBot.BP_TrackerBot_C" (Math|Transform|MakeTransform _array_element) "AdjustIfPossibleButDontSpawnIfColliding" 0 0))
        (Development|PrintString (Utilities|GetDisplayName _returnvalue))))))

(event EventSpawnNewBot
  (bind _returnvalue (AI|EQS|RunEQSQuery "/Game/Blueprints/EQS_FindSPawnLocation.EQS_FindSPawnLocation" self "RandomBest25Pct"))
  (EventDispatchers|AssignOnQueryFinishedEvent _returnvalue (delegate Custom|OnQueryFinishedEvent_Event_0)))

(fn ConstructionScript)